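; Inventory actor that stores item stacks in a fixed-size slot array and creates the main widget that displays them.
; AddItem tops up partial stacks of stackable items before seeking empty slots, while non-stackables take one slot each.
; It recurses to place overflow, returns any remainder that does not fit, and refreshes each changed slot widget by index.
; Helper functions query slot emptiness, amount and item info from class defaults.
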(event Custom|UpdateSlotAtIndex
  (params (Index :type Integer))
  (Default|UpdateSlot (Utilities|Array|Get(acopy) (Variables|/Game/Inventory/Blueprints/Widgets/Inventory.Inventory_C|GetSlotsWidgets (Variables|Default|GetInventory%20Widget)) Index)))

(event EventBeginPlay
  (Utilities|Array|Resize (Variables|Default|GetSlots) (Variables|Default|GetNumSlots))
  (bind _returnvalue (UserInterface|CreateWidget "/Game/Inventory/Blueprints/Widgets/MainWidget.MainWidget_C" 0 self (Variables|Default|GetSlotsPerRow)))
  (bind _output_get (Variables|Default|SetMainWidget _returnvalue))
  (Variables|Default|SetInventory%20Widget (Variables|/Game/Inventory/Blueprints/Widgets/MainWidget.MainWidget_C|GetInventoryWidget _output_get))
  (UserInterface|Viewport|AddtoViewport (Variables|Default|GetMainWidget) 0))

(event EventTick
  (params (DeltaSeconds :type Float%20%28single-precision%29)))

(fn ConstructionScript)

(fn IsSlotEmpty
  (params (Index :type Integer))
  (return (not (Utilities|IsValidClass (.ItemClass (Utilities|Struct|BreakS_InventorySlot (Utilities|Array|Get(acopy) (Variables|Default|GetSlots) Index)))))))

(fn GetItemInfoatIndex
  (params (Index :type Integer))
  (bind _slots (Variables|Default|GetSlots))
  (bind _output (Utilities|Array|Get(acopy) _slots Index))
  (bind (_itemclass _numitems) (Utilities|Struct|BreakS_InventorySlot _output))
  (if (Utilities|IsValidClass _itemclass)
    (return false (Utilities|GetClassDefaults _itemclass) _numitems)
    (else
      (return true "" 0))))

(fn SearchEmptySlot
  (bind _array_element (Utilities|Array|ForEachLoopwithBreak (Variables|Default|GetSlots) :!label _label)
    (:LoopBody
      (if (not (Utilities|IsValidClass (.ItemClass (Utilities|Struct|BreakS_InventorySlot _array_element))))
        (LocalVariables|SetlocalBool true)
        (LocalVariables|SetlocalIndex 0)
        (goto _label Break)))
    (:Completed
      (return (LocalVariables|GetlocalBool) (LocalVariables|GetlocalIndex)))))

(fn SearchFreeStack
  (params (ItemClass :type BP%20Inventory%20Item%20Class%20Reference))
  (bind (_array_element _array_index) (Utilities|Array|ForEachLoopwithBreak (Variables|Default|GetSlots) :!label _label)
    (:LoopBody
      (if (Utilities|IsValidClass (.ItemClass (Utilities|Struct|BreakS_InventorySlot _array_element)))
        (if (and (== (.ItemClass (Utilities|Struct|BreakS_InventorySlot _array_element)) ItemClass) (< (.NumItems (Utilities|Struct|BreakS_InventorySlot _array_element)) (Variables|Default|GetMaxStack)))
          (LocalVariables|SetlocalBool true)
          (LocalVariables|SetlocalIndex _array_index)
          (goto _label Break))))
    (:Completed
      (return (LocalVariables|GetlocalBool) (LocalVariables|GetlocalIndex)))))

(fn AddItem
  (params (ItemClass :type BP%20Inventory%20Item%20Class%20Reference) (Amount :type Integer))
  (LocalVariables|SetLocalClass ItemClass)
  (LocalVariables|SetLocalAmount Amount)
  (if (.CanStack (Utilities|Struct|BreakS_ItemInfo (Utilities|GetClassDefaults ItemClass)))
    (bind (_newparam _index) (CallFunction|SearchFreeStack (LocalVariables|GetLocalClass)))
    (if _newparam
      (bind _output_get (LocalVariables|SetFoundIndex _index))
      (if (> (+ (.numitems (Utilities|Array|Get(acopy) (Variables|Default|GetSlots) _output_get)) (LocalVariables|GetLocalAmount)) (Variables|Default|GetMaxStack))
        (LocalVariables|SetLocalAmount (- (+ (.numitems (Utilities|Array|Get(acopy) (Variables|Default|GetSlots) _output_get)) (LocalVariables|GetLocalAmount)) (Variables|Default|GetMaxStack)))
        (Utilities|Array|SetArrayElem (Variables|Default|GetSlots) (LocalVariables|GetFoundIndex) (Utilities|Struct|MakeS_InventorySlot (LocalVariables|GetLocalClass) (Variables|Default|GetMaxStack)))
        (CallFunction|UpdateSlotatIndex (LocalVariables|GetFoundIndex))
        (bind (_success _rest) (CallFunction|AddItem (LocalVariables|GetLocalClass) (LocalVariables|GetLocalAmount)))
        (return _success _rest)
        (else
          (Utilities|Array|SetArrayElem (Variables|Default|GetSlots) (LocalVariables|GetFoundIndex) (Utilities|Struct|MakeS_InventorySlot (LocalVariables|GetLocalClass) (+ (.numitems (Utilities|Array|Get(acopy) (Variables|Default|GetSlots) _output_get)) (LocalVariables|GetLocalAmount))))
          (CallFunction|UpdateSlotatIndex (LocalVariables|GetFoundIndex))
          (return true 0)))
      (else
        (bind (_success_2 _index_2) (CallFunction|SearchEmptySlot))
        (if _success_2
          (bind _output_get_2 (LocalVariables|SetFoundIndex _index_2))
          (if (> (LocalVariables|GetLocalAmount) (Variables|Default|GetMaxStack))
            (Utilities|Array|SetArrayElem (Variables|Default|GetSlots) _output_get_2 (Utilities|Struct|MakeS_InventorySlot (LocalVariables|GetLocalClass) (Variables|Default|GetMaxStack)))
            (CallFunction|UpdateSlotatIndex (LocalVariables|GetFoundIndex))
            (bind _rest_2 (CallFunction|AddItem (LocalVariables|GetLocalClass) (- (LocalVariables|GetLocalAmount) (Variables|Default|GetMaxStack))))
            (return true _rest_2)
            (else
              (Utilities|Array|SetArrayElem (Variables|Default|GetSlots) (LocalVariables|GetFoundIndex) (Utilities|Struct|MakeS_InventorySlot (LocalVariables|GetLocalClass) (LocalVariables|GetLocalAmount)))
              (CallFunction|UpdateSlotatIndex (LocalVariables|GetFoundIndex))
              (return true 0)))
          (else
            (return false (LocalVariables|GetLocalAmount))))))
    (else
      (bind (_success_3 _index_3) (CallFunction|SearchEmptySlot))
      (if _success_3
        (bind _output_get_3 (LocalVariables|SetFoundIndex _index_3))
        (Utilities|Array|SetArrayElem (Variables|Default|GetSlots) _output_get_3 (Utilities|Struct|MakeS_InventorySlot (LocalVariables|GetLocalClass) 1))
        (CallFunction|UpdateSlotatIndex (LocalVariables|GetFoundIndex))
        (if (> (LocalVariables|GetLocalAmount) 1)
          (bind _rest_3 (CallFunction|AddItem (LocalVariables|GetLocalClass) (- (LocalVariables|GetLocalAmount) 1)))
          (return true _rest_3)
          (else
            (return true 0)))
        (else
          (return false (LocalVariables|GetLocalAmount)))))))

(fn GetAmountatIndex
  (params (Index :type Integer))
  (return (.NumItems (Utilities|Struct|BreakS_InventorySlot (Utilities|Array|Get(acopy) (Variables|Default|GetSlots) Index)))))