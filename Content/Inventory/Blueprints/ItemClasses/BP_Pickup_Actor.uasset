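; BP_Pickup_Actor is a world item pickup that gives a set item and amount to an inventory on overlap.
; Its Sphere overlap casts the other actor to TestMech_Inventory and calls AddItem on that actor's inventory reference.
; On success, any leftover becomes the pickup's new Amount, allowing partial pickups; with nothing left, the actor destroys itself.
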(event OnComponentBeginOverlap(Sphere)
  (params (OverlappedComponent :type Primitive%20Component%20Object%20Reference) (OtherActor :type Actor%20Object%20Reference) (OtherComp :type Primitive%20Component%20Object%20Reference) (OtherBodyIndex :type Integer) (bFromSweep :type Boolean) (SweepResult :type Hit%20Result%20Structure%20%28by%20ref%29))
  (bind _astest_mech_inventory (Utilities|Casting|CastToTestMech_Inventory OtherActor))
  (Utilities|IsValid (Variables|/Game/MechStuff/TestMech_Inventory.TestMech_Inventory_C|GetInv_Ref _astest_mech_inventory)
    (:Is%20Valid
      (bind (_success _rest) (Default|AddItem (Variables|/Game/MechStuff/TestMech_Inventory.TestMech_Inventory_C|GetInv_Ref _astest_mech_inventory) (Variables|Default|GetItem%20To%20Add) (Variables|Default|GetAmount)))
      (if _success
        (if (> _rest 0)
          (Variables|Default|SetAmount _rest)
          (else
            (Actor|DestroyActor)))))))

(event EventBeginPlay)

(event Collision|EventActorBeginOverlap
  (params (OtherActor :type Actor%20Object%20Reference)))

(event EventTick
  (params (DeltaSeconds :type Float%20%28single-precision%29)))

(fn ConstructionScript)