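; HumanoidMech_BP is a player-controllable humanoid mech character with basic walking and jumping.
; MoveFB and MoveRL axis inputs add movement along forward and right vectors built from control yaw only, and SpaceBar triggers Jump.
; Both the construction script and BeginPlay hide the mesh's spine_01 bone and terminate its physics bodies, removing that bone chain from view in editor and at runtime.
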(event EventBeginPlay
  (|CallParentFunction)
  (Components|SkinnedMesh|HideBonebyName (Variables|Character|GetMesh) "spine_01" "PBO_Term"))

(event Collision|EventActorBeginOverlap
  (params (OtherActor :type Actor%20Object%20Reference)))

(event EventTick
  (params (DeltaSeconds :type Float%20%28single-precision%29)))

(event Input|AxisEvents|InputAxisMoveFB
  (params (AxisValue :type Float%20%28single-precision%29))
  (Pawn|Input|AddMovementInput (Math|Rotator|GetRotationXVector (Math|Rotator|MakeRotator 0.0 0.0 (.yaw (Pawn|GetControlRotation :!class /Script/Engine.Pawn)))) AxisValue false))

(event Input|AxisEvents|InputAxisMoveRL
  (params (AxisValue :type Float%20%28single-precision%29))
  (Pawn|Input|AddMovementInput (Math|Vector|GetRightVector (Math|Rotator|MakeRotator 0.0 0.0 (.yaw (Pawn|GetControlRotation :!class /Script/Engine.Pawn)))) AxisValue false))

(event Input|KeyboardEvents|SpaceBar
  (params (Key :type Key%20Structure :default "None"))
  (:Pressed
    (Character|Jump)))

(fn ConstructionScript
  (Components|SkinnedMesh|HideBonebyName (Variables|Character|GetMesh) "spine_01" "PBO_Term"))